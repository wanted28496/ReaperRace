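; Tombstone actor that rises into place when spawned and awards a point when its box overlaps an actor tagged "Grave".
; On BeginPlay, a timeline lerps the static mesh up from slightly below its origin, with mesh collision disabled for the first second.
; A tagged overlap calls IncreaseScore on the first TopDownCharacter found in the world, then destroys the tombstone.
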(event OnComponentBeginOverlap(Box)
  (params (OverlappedComponent :type Primitive%20Component%20Object%20Reference) (OtherActor :type Actor%20Object%20Reference) (OtherComp :type Primitive%20Component%20Object%20Reference) (OtherBodyIndex :type Integer) (bFromSweep :type Boolean) (SweepResult :type Hit%20Result%20Structure%20%28by%20ref%29))
  (if (Actor|ActorHasTag OtherActor "Grave")
    (bind _outactors (Actor|GetAllActorsOfClass "/Game/TopDownBP/Blueprints/TopDownCharacter.TopDownCharacter_C"))
    (bind _astop_down_character (Utilities|Casting|CastToTopDownCharacter (Utilities|Array|Get(acopy) _outactors)))
    (Default|IncreaseScore _astop_down_character)
    (Actor|DestroyActor)))

(event Custom|Grave%20Animation
  (bind _anim (Timeline|Anim Play)
    (:Update
      (Transformation|SetRelativeLocation (Variables|Default|GetStaticMesh) (Math|Vector|Lerp(Vector) "0, 0,-10.000000" "0, 0, 0" _anim) false false))))

(event EventBeginPlay
  (bind _staticmesh (Variables|Default|GetStaticMesh))
  (CallFunction|GraveAnimation)
  (Collision|SetCollisionEnabled _staticmesh "NoCollision")
  (Utilities|FlowControl|Delay 1.0)
  (Collision|SetCollisionEnabled _staticmesh "QueryAndPhysics"))

(fn ConstructionScript)